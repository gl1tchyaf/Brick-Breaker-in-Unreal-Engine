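; Ball actor for a paddle-and-ball game, reset to a fixed spot with a randomized heading when BallGameMode signals the start of play.
; While the game mode is in one specific state, Tick moves it by Direction times Speed in a swept offset, without delta-time scaling.
; Paddle hits reflect it, steered by paddle axis input and biased by MinX.
; Other hits simply reflect it and notify BallHitInterface actors.
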(event `self.ReceiveBeginPlay`
  (bind _asball_game_mode (cast `/Game/Blueprints/BallGameMode` (`GameplayStatics.GetGameMode`)))
  (add `/Game/Blueprints/BallGameMode.StartPlaying` _asball_game_mode (delegate `BallStartPlaying`)))

(event `BallStartPlaying`
  (`self.ResetBallPosition`))

(event `self.ReceiveTick`
  (params (DeltaSeconds :type "Float (single-precision)"))
  ;[1 1 1] Check state of the game
  (bind _asball_game_mode (cast `/Game/Blueprints/BallGameMode` (`GameplayStatics.GetGameMode`)))
  (if (`|EnumEquality` (`/Game/Blueprints/BallGameMode.StateOfTheGame` _asball_game_mode) "NewEnumerator5")
    (bind _sweephitresult (`self.K2_AddActorWorldOffset` (`KismetMathLibrary.MakeVector` (.x (* (`self.direction`) (`self.Speed`))) (.y (* (`self.direction`) (`self.Speed`)))) true))
    (bind (_bblockinghit _binitialoverlap _time _distance _location _impactpoint _normal _impactnormal _physmat _hitactor) (`GameplayStatics.BreakHitResult` _sweephitresult))
    (bind _aspaddle (cast `/Game/Blueprints/Paddle` _hitactor)
      (:`then`
        (bind _returnvalue (`KismetMathLibrary.GetReflectionVector` (`self.direction`) _impactnormal))
        (set `self.direction` (`KismetMathLibrary.Normal` (`KismetMathLibrary.MakeVector` (+ (`self.MinX`) (.x (`KismetMathLibrary.Normal` (`KismetMathLibrary.MakeVector` (.x _returnvalue) (+ (* (`/Game/Blueprints/Paddle.Axis Value` _aspaddle) 5.0) (.y _returnvalue)) (.z _returnvalue))))) (.y (`KismetMathLibrary.Normal` (`KismetMathLibrary.MakeVector` (.x _returnvalue) (+ (* (`/Game/Blueprints/Paddle.Axis Value` _aspaddle) 5.0) (.y _returnvalue)) (.z _returnvalue)))) (.z (`KismetMathLibrary.Normal` (`KismetMathLibrary.MakeVector` (.x _returnvalue) (+ (* (`/Game/Blueprints/Paddle.Axis Value` _aspaddle) 5.0) (.y _returnvalue)) (.z _returnvalue))))))))
      (:`CastFailed`
        (set `self.direction` _returnvalue)
        (if (`KismetSystemLibrary.DoesImplementInterface` _hitactor "/Game/Blueprints/BallHitInterface.BallHitInterface_C")
          (message `/Game/Blueprints/BallHitInterface.HitByBall` _hitactor))))))

(fn `ResetBallPosition`
  (`self.K2_SetActorLocation` (460.0 0.0 10.0))
  (set `self.direction` (`KismetMathLibrary.Normal` (`KismetMathLibrary.MakeVector` 1.0 (`KismetMathLibrary.RandomFloatInRange` -1.0 1.0)))))

(fn `UserConstructionScript`)