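; BallGameMode is a game mode Blueprint that holds the game's state and runs a three-second start countdown.
; BeginPlay sets the initial state, and StartCountdown resets the timer and switches to the countdown state.
; While in that state, Tick subtracts delta time, maps the remaining time to a 3-2-1 Count value, then advances to another state once the timer drops below zero.
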(event `self.ReceiveBeginPlay`
  (set `self.StateOfTheGame` "NewEnumerator0"))

(event `self.ReceiveTick`
  (params (DeltaSeconds :type "Float (single-precision)"))
  (if (`|EnumEquality` (`self.StateOfTheGame`) "NewEnumerator1")
    (bind _output_get (set `self.CountDown` (- (`self.CountDown`) DeltaSeconds)))
    (if (>= _output_get 2.0)
      (set `self.Count` 3)
      (elif (>= _output_get 1.0)
        (set `self.Count` 2)
        (elif (>= _output_get 0.0)
          (set `self.Count` 1)
          (else
            (set `self.StateOfTheGame` "NewEnumerator5")))))))

(event `StartCountdown`
  ;[1 1 1] Start countdown
  (set `self.CountDown` 3.0)
  (set `self.StateOfTheGame` "NewEnumerator1"))

(fn `UserConstructionScript`)